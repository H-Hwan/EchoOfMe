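; BP_Louver is a placeable actor that builds a row of repeated meshes, such as louver slats, in the level.
; Its construction script clears an InstancedStaticMesh component, assigns the chosen mesh and adds a set number of evenly spaced instances, so the result shows in the editor without playing.
; An enum selects the X, Y or Z axis, and a flag reverses the direction.
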(event `self.ReceiveBeginPlay`)

(fn `UserConstructionScript`
  (bind _instancedstaticmesh (`self.InstancedStaticMesh`))
  ; [Construction Script] - 게임을 실행하지 않아도 레벨 배치 단계에서 결과 확인 가능
  ; 메시 설정
  (`InstancedStaticMeshComponent.ClearInstances` _instancedstaticmesh)
  (`StaticMeshComponent.SetStaticMesh` _instancedstaticmesh (`self.StaticMesh`))
  ; Array Count만큼 반복
  (for _index (range (`self.Array Count`))
    ; 최종 배치
    (`InstancedStaticMeshComponent.AddInstance` (`self.InstancedStaticMesh`) (`KismetMathLibrary.MakeTransform` (* (* _index (`self.Distance`)) (* (select `/Game/Blueprint/RepeatArrangement/E_PlacementAxis` (`self.Placement Axis`) :`NewEnumerator0` (`self.X`) :`NewEnumerator1` (`self.Y`) :`NewEnumerator2` (`self.Z`)) (`KismetMathLibrary.SelectFloat` -1.0 1.0 (`self.bUseReverseDirection`))))) false)))