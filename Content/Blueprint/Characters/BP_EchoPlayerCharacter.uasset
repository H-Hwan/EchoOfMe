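; BP_EchoPlayerCharacter is the player character, with flashlight and listening abilities driven by Enhanced Input.
; The flashlight input toggles the Flashlight component, while holding the listen input starts and releasing it stops the Listening component.
; The Listening component reports state changes through an event bound at BeginPlay, which halves the cached walk speed while listening and restores it afterward.
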(event `self.ReceiveBeginPlay`
  ; Binding Event
  (add `ListeningComponent.OnListeningChanged` (`self.Listening`) (delegate `HandleListeningChanged`))
  (set `self.WalkSpeed` (`CharacterMovementComponent.MaxWalkSpeed` (`self.CharacterMovement`))))

(event `EnhancedInput|/Game/Input/Actions/IA_Flashlight`
  (params (ActionValue :type Boolean) (ElapsedSeconds :type "Float (double-precision)") (TriggeredSeconds :type "Float (double-precision)") (InputAction :type "InputAction Object Reference" :default "/Game/Input/Actions/IA_Flashlight.IA_Flashlight"))
  ; FlashLight Input
  (:`Started`
    (`FlashlightComponent.ToggleFlashLight` (`self.Flashlight`))))

(event `HandleListeningChanged`
  (params (bIsListening :type Boolean))
  (bind _walkspeed (`self.WalkSpeed`))
  ; Binding Event
  (set `CharacterMovementComponent.MaxWalkSpeed` (select `bool` bIsListening :`false` _walkspeed :`true` (* _walkspeed 0.5) :!type "Float (single-precision)") (`self.CharacterMovement`)))

(event `EnhancedInput|/Game/Input/Actions/IA_Listen`
  (params (ActionValue :type Boolean) (ElapsedSeconds :type "Float (double-precision)") (TriggeredSeconds :type "Float (double-precision)") (InputAction :type "InputAction Object Reference" :default "/Game/Input/Actions/IA_Listen.IA_Listen"))
  (bind _listening (`self.Listening`))
  ; Listen Input
  (:`Triggered`
    (`ListeningComponent.StartListening` _listening))
  (:`Completed`
    (`ListeningComponent.StopListening` _listening)))

(fn `UserConstructionScript`)