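; An actor component, meant for an EchoPlayerController owner, that creates and toggles the player's inventory UI.
; On BeginPlay it looks up the "Inventory"-tagged component on the player character, then overwrites it with the same lookup on its owner.
; It binds that to a new inventory widget, added to the viewport collapsed.
; ToggleInventory flips widget visibility, switching mouse cursor and input mode between Game-and-UI and Game-only.
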(event `self.ReceiveBeginPlay`
  (bind _inventorywidget (`self.InventoryWidget`))
  (`|ExecutionSequence`
    (:`then_0`
      ; Set Inventory Component
      (set `self.InventoryComp` (`Actor.FindComponentByTag` (`GameplayStatics.GetPlayerCharacter` 0) "/Script/EchoOfMe.InventoryComponent" "Inventory")))
    (:`then_1`
      ; Set Owner Controller
      (bind _asecho_player_controller (cast `EchoPlayerController` (`self.GetOwner`)))
      (set `self.OwnerController` _asecho_player_controller))
    (:`then_2`
      ; Set Inventory Component
      (set `self.InventoryComp` (`Actor.FindComponentByTag` (`self.GetOwner`) "/Script/EchoOfMe.InventoryComponent" "Inventory")))
    (:`then_3`
      ; Set Widget
      (bind _returnvalue (`|CreateWidget` (`self.InventoryClass`)))
      (bind _output_get (set `self.InventoryWidget` _returnvalue))
      (if (`KismetSystemLibrary.IsValid` _output_get)
        (`|ExecutionSequence`
          (:`then_0`
            (`InventoryWidget.BindInventory` _inventorywidget (`self.InventoryComp`)))
          (:`then_1`
            (`UserWidget.AddToViewport` _inventorywidget 0))
          (:`then_2`
            (`Widget.SetVisibility` _inventorywidget "Collapsed")))))))

(fn `ToggleInventory`
  (bind _inventorywidget (`self.InventoryWidget`))
  (bind _binventoryopen (`self.bInventoryOpen`))
  (bind _ownercontroller (`self.OwnerController`))
  (`KismetSystemLibrary.LogString` "LogTemp: Warning: [Toggle] ToggleInventory 호출됨")
  (`self.InventoryWidget`
    (:`then`
      (set `self.bInventoryOpen` (not (`self.bInventoryOpen`)))
      (`|ExecutionSequence`
        (:`then_0`
          (if _binventoryopen
            (`Widget.SetVisibility` _inventorywidget "Visible")
            (else
              (`Widget.SetVisibility` _inventorywidget "Collapsed"))))
        (:`then_1`
          (if _binventoryopen
            (`WidgetBlueprintLibrary.SetInputMode_GameAndUIEx` _ownercontroller null)
            (set `PlayerController.bShowMouseCursor` true _ownercontroller)
            (else
              (`WidgetBlueprintLibrary.SetInputMode_GameOnly` _ownercontroller)
              (set `PlayerController.bShowMouseCursor` false _ownercontroller))))))
    (:`else`)))